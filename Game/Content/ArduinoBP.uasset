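; Arduino input parser that turns a raw string into normalized controller axis values.
; Each Tick it extracts the text between the first two "s" markers of InputStr and splits it on commas.
; CreateArrays fills XValues and YValues with two repeated readings each, plus separate XControlStick and YControlStick values.
; Convert centers each reading on half of MaxValue, scales it and zeroes a small dead zone.
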(event EventTick
  (params (DeltaSeconds :type Float%20%28single-precision%29))
  (bind _inputstr (Variables|Default|GetInputStr))
  (bind (_lefts _rights _returnvalue) (Utilities|String|Split _inputstr "s"))
  (bind (_lefts_2 _rights_2 _returnvalue_2) (Utilities|String|Split _rights "s"))
  ;[1 1 1] Checks if string is valid
  (if _returnvalue
    (if _returnvalue_2
      (Variables|Default|SetFullValues _lefts_2)
      (CallFunction|CreateArrays))))

(fn ConstructionScript)

(fn CreateArrays
  (bind _fullvalues (Variables|Default|GetFullValues))
  (bind (_lefts _rights) (Utilities|String|Split _fullvalues ","))
  (bind (_lefts_2 _rights_2) (Utilities|String|Split _rights ","))
  (bind (_lefts_3 _rights_3) (Utilities|String|Split _rights_2 ","))
  (bind (_lefts_4 _rights_4) (Utilities|String|Split _rights_3 ","))
  (bind (_lefts_5 _rights_5) (Utilities|String|Split _rights_4 ","))
  (bind _newvalue (CallFunction|Convert _lefts))
  (bind _newvalue_2 (CallFunction|Convert _lefts_2))
  (bind _newvalue_3 (CallFunction|Convert _lefts_3))
  (Variables|Default|SetXControlStick _newvalue_3)
  (Variables|Default|SetXValues (Utilities|Array|MakeArray _newvalue _newvalue_2 _newvalue _newvalue_2))
  (bind _newvalue_4 (CallFunction|Convert _lefts_4))
  (bind _newvalue_5 (CallFunction|Convert _lefts_5))
  (bind _newvalue_6 (CallFunction|Convert (.LeftS (Utilities|String|Split _rights_5 ","))))
  (Variables|Default|SetYControlStick _newvalue_6)
  (Variables|Default|SetYValues (Utilities|Array|MakeArray _newvalue_4 _newvalue_5 _newvalue_4 _newvalue_5)))

(fn Convert
  (params (value :type String))
  (bind _returnvalue (Math|Conversions|ToFloat(Integer) value))
  (bind _maxvalue (Variables|Default|GetMaxValue))
  (bind _returnvalue_2 (/ _maxvalue 2.0))
  (bind _returnvalue_3 (- _returnvalue _returnvalue_2))
  (bind _returnvalue_4 (/ _returnvalue_3 _returnvalue_2))
  ;[1 1 1] If value is close to 0 it will be 0
  (if (< _returnvalue_4 0.1)
    (if (< -0.1 _returnvalue_4)
      (return 0.0)
      (else
        _)))
  (return _returnvalue_4))